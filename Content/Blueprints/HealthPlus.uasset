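; HealthPlus is a healing area that restores a BP_PlayerBase's Health while it stays inside the Collision component.
; Begin overlap sets PlayerInRadius and adds a quarter point immediately, then a Delay loop repeats every two seconds until Health reaches at least 1.0, without clamping.
; End overlap clears the flag, which the loop checks after each delay.
; The full-health branch only casts the player character; the IsAlive setter is disconnected.
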(event OnComponentBeginOverlap(Collision)
  (params (OverlappedComponent :type Primitive%20Component%20Object%20Reference) (OtherActor :type Actor%20Object%20Reference) (OtherComp :type Primitive%20Component%20Object%20Reference) (OtherBodyIndex :type Integer) (bFromSweep :type Boolean) (SweepResult :type Hit%20Result%20Structure%20%28by%20ref%29))
  (bind _asbp_player_base (Utilities|Casting|CastToBP_PlayerBase OtherActor))
  (Variables|Default|SetPlayerInRadius true)
  (bind _output_get (Variables|/Game/Blueprints/BP_PlayerBase.BP_PlayerBase_C|SetHealth _asbp_player_base (+ (Variables|/Game/Blueprints/BP_PlayerBase.BP_PlayerBase_C|GetHealth _asbp_player_base) 0.25) :!label _label))
  (if (>= _output_get 1.0)
    (bind _asbp_player_base_2 (Utilities|Casting|CastToBP_PlayerBase (Game|GetPlayerCharacter 0)))
    (else
      (Utilities|FlowControl|Delay 2.0)
      (if (Variables|Default|GetPlayerInRadius)
        (goto _label)))))

(event OnComponentEndOverlap(Collision)
  (params (OverlappedComponent :type Primitive%20Component%20Object%20Reference) (OtherActor :type Actor%20Object%20Reference) (OtherComp :type Primitive%20Component%20Object%20Reference) (OtherBodyIndex :type Integer))
  (Utilities|Casting|CastToBP_PlayerBase OtherActor)
  (Variables|Default|SetPlayerInRadius false))

(event EventBeginPlay)

(event Collision|EventActorBeginOverlap
  (params (OtherActor :type Actor%20Object%20Reference)))

(event EventTick
  (params (DeltaSeconds :type Float%20%28single-precision%29)))

(fn ConstructionScript)
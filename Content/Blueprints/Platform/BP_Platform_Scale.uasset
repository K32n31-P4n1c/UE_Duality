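; BP_Platform_Scale is a platform actor that animates its own scale during play.
; BeginPlay stores the starting 3D scale and sets a Start flag, which lets Tick call Play on a timeline every frame.
; Each timeline update sets the actor scale to the stored scale plus the track value, so the animation is an additive offset from the placed size.
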(event EventBeginPlay
  (Variables|Default|SetScaleOfPlatform (Transformation|GetActorScale3D))
  (Variables|Default|SetStart true))

(event EventTick
  (params (DeltaSeconds :type Float%20%28single-precision%29))
  (if (Variables|Default|GetStart)
    (Utilities|FlowControl|Sequence
      (:then_0
        (bind _newtrack_0 (Timeline|Timeline_0 Play)
          (:Update
            (Transformation|SetActorScale3D (+ _newtrack_0 (Variables|Default|GetScaleOfPlatform)))))))))

(fn ConstructionScript)
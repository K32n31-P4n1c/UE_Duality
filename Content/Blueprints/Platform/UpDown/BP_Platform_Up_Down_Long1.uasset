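; A long platform actor that moves up and down from the position where it is placed.
; BeginPlay stores the starting location and sets a start flag.
; While the flag is set, Tick calls Play on a timeline, whose vector track is added to the stored location and applied with SetActorLocation, without sweep.
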(event EventBeginPlay
  (Variables|Default|SetLocationOfPlatform (Transformation|GetActorLocation))
  (Variables|Default|SetStart true))

(event EventTick
  (params (DeltaSeconds :type Float%20%28single-precision%29))
  (if (Variables|Default|GetStart)
    (Utilities|FlowControl|Sequence
      (:then_0
        (bind _newtrack_0 (Timeline|Timeline_0 Play)
          (:Update
            (Transformation|SetActorLocation (+ _newtrack_0 (Variables|Default|GetLocationOfPlatform)) false false)))))))

(fn ConstructionScript)
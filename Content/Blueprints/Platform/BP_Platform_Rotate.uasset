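; Platform actor that rotates in pitch, driven by a timeline.
; BeginPlay stores the starting rotation in LocationOfPlatform and sets a Start flag, which lets Tick call Play on the timeline every frame.
; Each timeline update adds the track value to the starting pitch and applies it as the actor rotation, forcing roll and yaw to zero.
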(event EventBeginPlay
  (Variables|Default|SetLocationOfPlatform (Transformation|GetActorRotation))
  (Variables|Default|SetStart true))

(event EventTick
  (params (DeltaSeconds :type Float%20%28single-precision%29))
  (if (Variables|Default|GetStart)
    (Utilities|FlowControl|Sequence
      (:then_0
        (bind _newtrack_0 (Timeline|Timeline_0 Play)
          (:Update
            (Transformation|SetActorRotation (Math|Rotator|MakeRotator 0.0 (+ _newtrack_0 (.Pitch (Math|Rotator|BreakRotator (Variables|Default|GetLocationOfPlatform)))) 0.0))
            (for _index (range 0 0)
              _)))))))

(fn ConstructionScript)